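; BP_StoryGenerator builds procedural story text from agents, items and actions defined in data tables.
; On BeginPlay it parses the three tables and expands the action list with item interaction actions.
; Each GenerateLine call passes actions and agents to PrintGeneratedStory, stores the returned agent state and appends the new line.
; Text getters expose the data and story, while clearing the story re-imports agents to reset their state.
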(event EventBeginPlay
  (CallFunction|ImportAll))

(fn ConstructionScript)

(fn GetActionsText
  (for _array_element (Variables|Default|GetActions)
    (LocalVariables|SetText (Utilities|String|Append (LocalVariables|GetText) (Utilities|String|Append (Utilities|Struct|BreakAction _array_element) " 
"))))
  (return (Utilities|Text|ToText(String) (LocalVariables|GetText))))

(fn GetAgentsText
  (for _array_element (Variables|Default|GetAgents)
    (LocalVariables|SetTraits "")
    (for _array_element_2 (.m_Attributes (Utilities|Struct|BreakAgentState _array_element))
      (if (Utilities|Array|IsEmpty (LocalVariables|GetTraits))
        (LocalVariables|SetTraits (Utilities|Struct|BreakAttribute _array_element_2))
        (else
          (LocalVariables|SetTraits (Utilities|String|Append (LocalVariables|GetTraits) ", " (Utilities|Struct|BreakAttribute _array_element_2))))))
    (LocalVariables|SetText (Utilities|String|Append (LocalVariables|GetText) (Utilities|String|Append (.m_Name (Utilities|Struct|BreakAgentState _array_element)) " (" (LocalVariables|GetTraits) ")" " 
"))))
  (return (Utilities|Text|ToText(String) (LocalVariables|GetText))))

(fn GetItemsText
  (for _array_element (Variables|Default|GetItems)
    (LocalVariables|SetText (Utilities|String|Append (LocalVariables|GetText) (Utilities|String|Append (Utilities|Struct|BreakItem _array_element) " 
"))))
  (return (Utilities|Text|ToText(String) (LocalVariables|GetText))))

(fn GenerateLine
  (bind (_storyline _returnvalue) (Class|BehaviorGeneratorFunctionLibrary|PrintGeneratedStory (Variables|Default|GetActions) (Variables|Default|GetAgents)))
  (Variables|Default|SetAgents _returnvalue)
  (if (Utilities|Array|IsEmpty (Variables|Default|GetStoryLines))
    (Variables|Default|SetStoryLines (Utilities|String|Append _storyline " 
"))
    (else
      (Variables|Default|SetStoryLines (Utilities|String|Append (Variables|Default|GetStoryLines) (Utilities|String|Append _storyline " 
"))))))

(fn GetStoryLines
  (return (Variables|Default|GetStoryLines)))

(fn ClearStoryLines
  (Variables|Default|SetStoryLines "")
  (CallFunction|ImportAgents))

(fn ImportAll
  (CallFunction|ImportAgents)
  (bind _returnvalue (Class|BehaviorGeneratorFunctionLibrary|ParseItems (Variables|Default|GetItems%20DT)))
  (Variables|Default|SetItems _returnvalue)
  (bind _returnvalue_2 (Class|BehaviorGeneratorFunctionLibrary|ParseActions (Variables|Default|GetActions%20DT)))
  (bind _returnvalue_3 (Class|BehaviorGeneratorFunctionLibrary|AddItemInteractionActions (Variables|Default|GetItems) _returnvalue_2))
  (Variables|Default|SetActions _returnvalue_3))

(fn ImportAgents
  (bind _returnvalue (Class|BehaviorGeneratorFunctionLibrary|ParseAgents (Variables|Default|GetAgents%20DT)))
  (Variables|Default|SetAgents _returnvalue))